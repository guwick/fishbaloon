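; BP_Character is a player-controlled pawn that moves around and drops bombs.
; The Naprej nazaj (forward/back) and levo desno (left/right) axes add movement input along vectors derived from control yaw only, ignoring pitch and roll.
; The Spawnbomb press spawns a BP_bomba slightly below the actor's location, regardless of collisions.
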(event `InputAction|Spawnbomb`
  (params (Key :type "Key Structure"))
  (bind (_returnvalue_x _returnvalue_y _returnvalue_z) (`KismetMathLibrary.BreakVector` (`self.K2_GetActorLocation`)))
  (:`Pressed`
    (`|SpawnActorFromClass` "/Game/Blueprints/BP_bomba.BP_bomba_C" (`KismetMathLibrary.MakeTransform` (`KismetMathLibrary.MakeVector` _returnvalue_x _returnvalue_y (- _returnvalue_z 40.0))) "AlwaysSpawn" "OverrideRootScale" null null)))

(event `InputAxis|Naprej nazaj`
  (params (AxisValue :type "Float (single-precision)"))
  ;[1 1 1] movement
  (`self.AddMovementInput` (`KismetMathLibrary.GetForwardVector` (`KismetMathLibrary.MakeRotator` 0.0 0.0 (.yaw (`self.GetControlRotation`)))) AxisValue))

(event `InputAxis|levo desno`
  (params (AxisValue :type "Float (single-precision)"))
  ;[1 1 1] movement
  (`self.AddMovementInput` (`KismetMathLibrary.GetRightVector` (`KismetMathLibrary.MakeRotator` 0.0 0.0 (.yaw (`self.GetControlRotation`)))) AxisValue))

(fn `UserConstructionScript`)