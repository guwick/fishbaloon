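; Explosion actor for a bomb that reaches as far as the bomb's owning character's Range and clears what it hits.
; On BeginPlay it saves that range, destroys the bomb, and box-traces along the up vector of four meshes.
; Each mesh stretches to its first hit or full range; hit bombs chain-explode, while characters, terrain and pickups are destroyed.
; The explosion removes itself after a short delay.
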(event `self.ReceiveBeginPlay`
  (bind _hitactor (`self.hitactor`))
  (`|ExecutionSequence`
    (:`then_0`
      ;[1 1 1] set explosion range
      (set `self.rangesave` (`/Game/Blueprints/BP_Character.range` (`/Game/Blueprints/BP_bomba.character` (`self.bomba`)))))
    (:`then_1`
      ;[1 1 1] destory parent bomb
      (`self.K2_DestroyActor` (`self.bomba`))
      (`|ExecutionSequence`
        (:`then_0`
          ;[1 1 1] boxtrace za vse meshe
          (for _array_element (`|MakeArray` (`self.w`) (`self.w1`) (`self.w2`) (`self.w3`) :!type "SceneComponent Object Reference")
            (bind _returnvalue (`SceneComponent.K2_GetComponentLocation` _array_element))
            (bind _outhit (`KismetSystemLibrary.BoxTraceSingle` _returnvalue (+ _returnvalue (* (`SceneComponent.GetUpVector` _array_element) (- (`self.rangesave`) 25.0))) (25.0 25.0 25.0) (struct) "TraceTypeQuery1" false (`|MakeArray` (`self.bomba`) :!type "Actor Object Reference") "ForDuration"))
            ;[1 1 1] scale za meshe
            (set `self.hitactor` (`.HitActor` (`GameplayStatics.BreakHitResult` _outhit)))
            (`SceneComponent.SetRelativeScale3D` _array_element (`KismetMathLibrary.MakeVector` 0.25 0.25 (/ (`KismetMathLibrary.SelectFloat` (`.Distance` (`GameplayStatics.BreakHitResult` _outhit)) (`self.rangesave`) (`GameplayStatics.BreakHitResult` _outhit)) 200.0)))
            ;[1 1 1] destroy other actor
            (`|ExecutionSequence`
              (:`then_0`
                (bind _asbp_bomba (cast `/Game/Blueprints/BP_bomba` _hitactor))
                (`/Game/Blueprints/BP_bomba.chainexplosion` _asbp_bomba))
              (:`then_1`
                (bind _asbp_character (cast `/Game/Blueprints/BP_Character` _hitactor))
                (`self.K2_DestroyActor` _asbp_character))
              (:`then_2`
                (bind _asbp_terrain (cast `/Game/Blueprints/BP_terrain` _hitactor))
                (`self.K2_DestroyActor` _asbp_terrain))
              (:`then_3`
                (bind _asbp_pickup (cast `/Game/Blueprints/BP_pickup` _hitactor))
                (`self.K2_DestroyActor` _asbp_pickup)))))
        (:`then_1`
          ;[1 1 1] destory self
          (`KismetSystemLibrary.Delay` 0.5)
          (`self.K2_DestroyActor`))))))

(fn `UserConstructionScript`)