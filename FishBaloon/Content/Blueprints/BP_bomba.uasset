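; BP_bomba is a timed bomb placed by a character that detonates after a short fuse.
; Detonation decrements the character's STbomb counter and spawns BP_explosion at the bomb's location, passing itself as Bomba.
; The chainexplosion event jumps straight into that detonation path, skipping the delay.
; When a BP_Character leaves the Sphere overlap, the bomb enables blocking collision as a non-simulated WorldDynamic object.
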(event `self.ReceiveBeginPlay`
  (`KismetSystemLibrary.Delay` 3.0)
  ;[1 1 1] STbomb --
  (`/Engine/EditorBlueprintResources/StandardMacros.DecrementInt` (`/Game/Blueprints/BP_Character.STbomb` (`self.character`)) :!label _label
    (:`  `
      ;[1 1 1] spawn bomb
      (`|SpawnActorFromClass` "/Game/Blueprints/BP_explosion.BP_explosion_C" (`KismetMathLibrary.Conv_VectorToTransform` (`self.K2_GetActorLocation`)) "AlwaysSpawn" "OverrideRootScale" null self null))))

(event `chainexplosion`
  (goto _label))

(event `self.Sphere.OnComponentEndOverlap`
  (params (OverlappedComponent :type "PrimitiveComponent Object Reference") (OtherActor :type "Actor Object Reference") (OtherComp :type "PrimitiveComponent Object Reference") (OtherBodyIndex :type Integer))
  (bind _sphere (`self.Sphere`))
  (bind _sphere_2 (`self.Sphere`))
  ;[1 1 1] enable collision after character leaves
  (cast `/Game/Blueprints/BP_Character` OtherActor)
  (`PrimitiveComponent.SetSimulatePhysics` _sphere false)
  (`self.SetActorEnableCollision` true)
  (`PrimitiveComponent.SetCollisionEnabled` _sphere "QueryAndPhysics")
  (`PrimitiveComponent.SetCollisionResponseToAllChannels` _sphere_2 "ECR_Block")
  (`PrimitiveComponent.SetCollisionObjectType` _sphere_2 "ECC_WorldDynamic")
  (`PrimitiveComponent.SetCollisionObjectType` _sphere "ECC_WorldDynamic"))

(fn `UserConstructionScript`)