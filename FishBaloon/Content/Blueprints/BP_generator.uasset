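; BP_generator fills a grid with BP_terrain blocks at BeginPlay, forming the level's terrain around pre-placed walls.
; It caches BP_undestructible locations and skips cells whose centre exactly matches one, using the Offset spacing from its own position.
; After each column, inside the outer loop, it calls ClearArea on every BP_spawnArea and GenerateAllPickups on PickupManager, so both repeat per column.
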(event `self.ReceiveBeginPlay`
  (bind _returnvalue (/ (`self.offset`) 2))
  ;[1 1 1] Spawning walls
  (bind _outactors (`GameplayStatics.GetAllActorsOfClass` "/Game/Blueprints/BP_undestructible.BP_undestructible_C"))
  (for _array_element _outactors
    (`KismetArrayLibrary.Array_Add` (`self.walls`) (`self.K2_GetActorLocation` _array_element)))
  (for _index (range (+ (`self.Xlength`) 1))
    (for _index_2 (range (+ (`self.Ylength`) 1))
      (bind _returnvalue_2 (+ (`self.K2_GetActorLocation`) (`KismetMathLibrary.MakeVector` (`KismetMathLibrary.Conv_IntToDouble` (+ (* _index (`self.offset`)) _returnvalue)) (`KismetMathLibrary.Conv_IntToDouble` (+ (* _index_2 (`self.offset`)) _returnvalue)))))
      (if (== (`KismetArrayLibrary.Array_Find` (`self.walls`) _returnvalue_2) -1)
        (`|SpawnActorFromClass` "/Game/Blueprints/BP_terrain.BP_terrain_C" (`KismetMathLibrary.MakeTransform` _returnvalue_2) "Undefined" "OverrideRootScale" null null)))
    (bind _outactors_2 (`GameplayStatics.GetAllActorsOfClass` "/Game/Blueprints/BP_spawnArea.BP_spawnArea_C"))
    (for _array_element_2 _outactors_2
      (`/Game/Blueprints/BP_spawnArea.ClearArea` _array_element_2))
    (`/Game/Blueprints/BP_pickup_manager.GenerateAllPickups` (`self.pickupManager`))))

(fn `UserConstructionScript`)