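; BP_pickup_manager assigns pickups to terrain actors in the level when GenerateAllPickups is called.
; It gathers every BP_terrain actor, shuffles the list, then gives as many tiles as each MaxBomb count specifies the matching Pickups entry and flags them as holding a pickup.
; A running terrain index keeps each tile to one pickup and stops assignment when tiles run out.
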(event `GenerateAllPickups`
  (bind _terraini (`self.terrainI`))
  (bind _output (`|GetArrayItem` (`self.Terrain`) _terraini))
  (bind _returnvalue (== (`self.terrainI`) (`KismetArrayLibrary.Array_Length` (`self.Terrain`))))
  (bind _outactors (`GameplayStatics.GetAllActorsOfClass` "/Game/Blueprints/BP_terrain.BP_terrain_C"))
  (bind _output_get (set `self.Terrain` _outactors))
  (`KismetArrayLibrary.Array_Shuffle` _output_get)
  (for (_array_element _array_index) (`self.maxBomb`) :!label _label
    (`KismetSystemLibrary.PrintString` (`KismetStringLibrary.Conv_IntToString` _array_element))
    (for _ (range 1 (+ _array_element 1))
      (if _returnvalue
        (goto _label :!via `Break`)
        (else
          (set `/Game/Blueprints/BP_terrain.pickups` (`|GetArrayItem` (`self.pickups`) _array_index) _output)
          (set `/Game/Blueprints/BP_terrain.hasPickup` true _output)
          (`/Engine/EditorBlueprintResources/StandardMacros.IncrementInt` _terraini
            (:`  `
              (if _returnvalue
                (goto _label :!via `Break`)))))))))

(event `self.ReceiveBeginPlay`)

(fn `UserConstructionScript`)